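; Spline-based race track generator that builds the track in the editor and handles AI waypoints and lap completion.
; The construction script syncs per-point road data, then lays banked, scaled spline meshes for road and optional guard rails.
; It also adds optional point-number labels and sizes the finish volume.
; WaypointSetup spawns linked waypoints at spline points; finish overlaps report player and AI laps to the game mode.
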(event `self.ReceiveBeginPlay`)

(event `WaypointSetup`
  ;[1 1 1] Add waypoints for the AI to take and set them up.
  (for _index (range (+ (`SplineComponent.GetNumberOfSplinePoints` (`self.Spline`)) 1))
    (bind _returnvalue (`|SpawnActorFromClass` "/Game/Blueprints/Core/RacingWaypoint.RacingWaypoint_C" (`SplineComponent.GetTransformAtSplinePoint` (`self.Spline`) _index "World" false) "Undefined" "OverrideRootScale" null null))
    (`KismetArrayLibrary.Array_Add` (`self.Waypoints`) _returnvalue))
  (for (_array_element _array_index) (`self.Waypoints`)
    (bind _returnvalue_2 (+ _array_index 1))
    (set `RacingAI_Waypoint.NextWaypoint` (`|GetArrayItem` (`self.Waypoints`) (`KismetMathLibrary.SelectInt` 1 _returnvalue_2 (>= _returnvalue_2 (`KismetArrayLibrary.Array_Length` (`self.Waypoints`))))) _array_element)))

(event `self.FinishVolume.OnComponentBeginOverlap`
  (params (OverlappedComponent :type "PrimitiveComponent Object Reference") (OtherActor :type "Actor Object Reference") (OtherComp :type "PrimitiveComponent Object Reference") (OtherBodyIndex :type Integer) (bFromSweep :type Boolean) (SweepResult :type "HitResult Structure (by ref)"))
  (bind _vehicleadvancedgamemode (`/Game/Blueprints/Core/RacingFunctionLibrary.GetVehicleGameMode`))
  ;[1 1 1] When the player passes through the collider, complete the lap
  (if (`self.StartingTrack`)
    (bind _asbp_celica (cast `/Game/Vehicles/Celica/BP_Celica` OtherActor)
      (:`then`
        (if (== (`/Game/Vehicles/00_Master_Vehicle/BP_Master_Vehicle.Driver TriggerBox` _asbp_celica) OtherComp)
          (`/Game/Blueprints/Core/VehicleAdvGameMode.PlayerFinishLine` _vehicleadvancedgamemode)
          (`self.LapCompleted` true (`/Game/Blueprints/Core/VehicleAdvGameMode.Current Laps` _vehicleadvancedgamemode))))
      (:`CastFailed`
        (bind _asvehicle_bmai_race (cast `/Game/Blueprints/Tools/Vehicle_BMAI_Race` OtherActor))
        (if (== (`Actor.RootComponent` _asvehicle_bmai_race) OtherComp)
          (`/Game/Blueprints/Core/VehicleAdvGameMode.AIFinishLine` (`/Game/Blueprints/Core/RacingFunctionLibrary.GetVehicleGameMode`) _asvehicle_bmai_race)
          (`self.LapCompleted` false (`/Game/Blueprints/Tools/Vehicle_BMAI_Race.Laps` _asvehicle_bmai_race)))))))

(fn `BuildTrackElements`
  (params (LoopIndex :type Integer) (TrackElementMesh :type "StaticMesh Object Reference"))
  (locals (Local_CurrentLoopIndex :type Integer) (Local_NextLoopIndex :type Integer) (Local_TrackElementMesh :type "StaticMesh Object Reference") (Local_StartLocation :type "Vector Structure") (Local_StartTangent :type "Vector Structure") (Local_EndLocation :type "Vector Structure") (Local_EndTangent :type "Vector Structure") (Local_CurrentSplineMesh :type "SplineMeshComponent Object Reference") (Local_StartRoll :type "Float (double-precision)") (Local_StartScale :type "Vector2D Structure") (Local_EndRoll :type "Float (double-precision)") (Local_EndScale :type "Vector2D Structure"))
  (bind (_location _tangent) (`SplineComponent.GetLocationAndTangentAtSplinePoint` (`self.Spline`) (`local.Local_NextLoopIndex`) "Local"))
  (bind (_location_2 _tangent_2) (`SplineComponent.GetLocationAndTangentAtSplinePoint` (`self.Spline`) (`local.Local_CurrentLoopIndex`) "Local"))
  (bind (_output_leftguardrail _output_rightguardrail _output_trackbank _output_trackwidth _output_trackthickness) (break `/Game/Blueprints/Data/RoadData` (`|GetArrayItem` (`self.RoadDataArray`) (`local.Local_CurrentLoopIndex`))))
  (bind (_output_leftguardrail_2 _output_rightguardrail_2 _output_trackbank_2 _output_trackwidth_2 _output_trackthickness_2) (break `/Game/Blueprints/Data/RoadData` (`|GetArrayItem` (`self.RoadDataArray`) (`local.Local_NextLoopIndex`))))
  ;[1 1 1] Determines the current and next spline points.
  (set `local.Local_CurrentLoopIndex` LoopIndex)
  (set `local.Local_NextLoopIndex` (mod (+ LoopIndex 1) (`self.NumberOfSplinePoints`)))
  ;[1 1 1] Sets the mesh to place here.
  (set `local.Local_TrackElementMesh` TrackElementMesh)
  ;[1 1 1] Sequence because we make our code easy to read
  (`|ExecutionSequence`
    (:`then_0`
      ;[1 1 1] Gets the location and tangent (basically direction) of the first spline point.
      (set `local.Local_StartLocation` _location_2)
      (set `local.Local_StartTangent` _tangent_2)
      ;[1 1 1] <- Same as before, but with the next spline point.
      (set `local.Local_EndLocation` _location)
      (set `local.Local_EndTangent` _tangent)
      ;[1 1 1] Gets the roll and size for the start of the mesh from the road data array
      (set `local.Local_StartRoll` _output_trackbank)
      (set `local.Local_StartScale` (`KismetMathLibrary.MakeVector2D` _output_trackwidth _output_trackthickness))
      ;[1 1 1] Same as before, but for the end of the mesh.
      (set `local.Local_EndRoll` _output_trackbank_2)
      (set `local.Local_EndScale` (`KismetMathLibrary.MakeVector2D` _output_trackwidth_2 _output_trackthickness_2)))
    (:`then_1`
      ;[1 1 1] Creates the spline mesh component.
      (bind _returnvalue (`AddComponent|NODE_AddSplineMeshComponent-0`))
      (set `local.Local_CurrentSplineMesh` _returnvalue)
      ;[1 1 1] Assigns the track mesh to it.
      (`StaticMeshComponent.SetStaticMesh` (`local.Local_CurrentSplineMesh`) (`local.Local_TrackElementMesh`))
      ;[1 1 1] Sets the location and tangent for both ends of the mesh.
      (`SplineMeshComponent.SetStartAndEnd` (`local.Local_CurrentSplineMesh`) (`local.Local_StartLocation`) (`local.Local_StartTangent`) (`local.Local_EndLocation`) (`local.Local_EndTangent`) true)
      ;[1 1 1] Sets the roll for the mesh at both start and end.
      (`SplineMeshComponent.SetStartRoll` (`local.Local_CurrentSplineMesh`) (`local.Local_StartRoll`) true)
      (`SplineMeshComponent.SetEndRoll` (`local.Local_CurrentSplineMesh`) (`local.Local_EndRoll`) true)
      ;[1 1 1] Sets the scale for the mesh at both the start and the end.
      (`SplineMeshComponent.SetStartScale` (`local.Local_CurrentSplineMesh`) (`local.Local_StartScale`) true)
      (`SplineMeshComponent.SetEndScale` (`local.Local_CurrentSplineMesh`) (`local.Local_EndScale`) true)
      ;[1 1 1] If collisions are enabled then make sure that the mesh has them.
      (`PrimitiveComponent.SetCollisionEnabled` (`local.Local_CurrentSplineMesh`) (select `bool` (`self.Collisions`) :`false` "NoCollision" :`true` "QueryAndPhysics" :!type "ECollisionEnabled Enum"))
      ;[1 1 1] Change the properties of the railing mesh
      (if (!= (`local.Local_CurrentSplineMesh`) (`self.RoadMesh`))
        (`PrimitiveComponent.SetCollisionResponseToChannel` (`local.Local_CurrentSplineMesh`) "ECC_GameTraceChannel2" "ECR_Block")
        (`PrimitiveComponent.SetCollisionResponseToChannel` (`local.Local_CurrentSplineMesh`) "ECC_GameTraceChannel1" "ECR_Block")))))

(fn `UserConstructionScript`
  (locals (FinishHalfHeight :type "Float (double-precision)" :default 0.0))
  (bind _roaddataarray (`self.RoadDataArray`))
  (bind (_output_leftguardrail _output_rightguardrail) (break `/Game/Blueprints/Data/RoadData` (`|GetArrayItem` (`self.RoadDataArray`) (`self.CurrentLoopIndex`))))
  (bind (_output_leftguardrail_2 _output_rightguardrail_2 _output_trackbank _output_trackwidth) (break `/Game/Blueprints/Data/RoadData` (`|GetArrayItem` (`self.RoadDataArray`) (`self.StartLocation`))))
  (bind (_output_leftguardrail_3 _output_rightguardrail_3 _output_trackbank_2 _output_trackwidth_2 _output_trackthickness _output_sandroad) (break `/Game/Blueprints/Data/RoadData` (`|GetArrayItem` (`self.RoadDataArray`) (`self.CurrentLoopIndex`))))
  (bind _returnvalue (* (1000.0 700.0 215.0) _output_trackwidth))
  ;[1 1 1] Disables the entire construction script if build track is disabled.
  (if (`self.BuildTrack`)
    (`|ExecutionSequence`
      (:`then_0`
        ;[1 1 1] Count how many points are on the spline.
        (set `self.NumberOfSplinePoints` (`SplineComponent.GetNumberOfSplinePoints` (`self.Spline`))))
      (:`then_1`
        ;[1 1 1] Makes sure the road data array matches the spline length
        (`/Engine/EditorBlueprintResources/StandardMacros.CompareInt` (`KismetArrayLibrary.Array_Length` (`self.RoadDataArray`)) (`self.NumberOfSplinePoints`) :!label _label
          (:`>`
            (`KismetArrayLibrary.Array_Remove` _roaddataarray (`KismetArrayLibrary.Array_LastIndex` _roaddataarray))
            (goto _label))
          (:`<`
            (`KismetArrayLibrary.Array_Add` (`self.RoadDataArray`) (`self.RoadMeshDefaults`))
            (goto _label))))
      (:`then_2`
        ;[1 1 1] Initializing variables for placing the meshes.
        (for _index (range (+ (- (`self.NumberOfSplinePoints`) (`KismetMathLibrary.SelectInt` 1 2 (`self.LoopingTrack`))) 1))
          (set `self.CurrentLoopIndex` _index)
          (set `self.DrawLeftGuardRail` _output_leftguardrail)
          (set `self.DrawRightGuardRail` _output_rightguardrail)
          ;[1 1 1] Another sequence, since this section of the blueprint does 3 different things.
          (`|ExecutionSequence`
            (:`then_0`
              ;[1 1 1] Place the road mesh
              (`self.BuildTrackElements` (`self.CurrentLoopIndex`) (select `bool` _output_sandroad :`false` (`self.RoadMesh`) :`true` (`self.OffRoadMesh`))))
            (:`then_1`
              ;[1 1 1] Place the left rails
              (if (and (`self.DrawLeftGuardRail`) (`self.BuildRails`))
                (`self.BuildTrackElements` (`self.CurrentLoopIndex`) (`self.LeftGuardRailMesh`))))
            (:`then_2`
              ;[1 1 1] Place the right rails
              (if (and (`self.DrawRightGuardRail`) (`self.BuildRails`))
                (`self.BuildTrackElements` (`self.CurrentLoopIndex`) (`self.RightGuardRailMesh`)))))))
      (:`then_3`
        ;[1 1 1] Labels points on the track.
        (if (`self.DrawTrackPointNumbers`)
          (for _index_2 (range (`self.NumberOfSplinePoints`))
            (set `self.CurrentTrackPoint` (`KismetStringLibrary.Conv_IntToString` _index_2))
            (bind (_location _tangent) (`SplineComponent.GetLocationAndTangentAtSplinePoint` (`self.Spline`) _index_2 "Local"))
            (bind _returnvalue_2 (`AddComponent|NODE_AddTextRenderComponent-0` :`RelativeTransform` (`KismetMathLibrary.MakeTransform` (`KismetMathLibrary.MakeVector` (.x _location) (.y _location) (+ (.z _location) 50.0)) (`KismetMathLibrary.Conv_VectorToRotator` (* _tangent -1.0)))))
            (`TextRenderComponent.K2_SetText` _returnvalue_2 (`KismetTextLibrary.Conv_StringToText` (`self.CurrentTrackPoint`))))))
      (:`then_5`
        ;[1 1 1] Set the finish line
        (`BoxComponent.SetBoxExtent` (`self.FinishVolume`) _returnvalue false)
        (set `local.FinishHalfHeight` (/ (.z _returnvalue) 2.0))
        (`SceneComponent.K2_SetWorldLocationAndRotation` (`self.FinishVolume`) (`KismetMathLibrary.MakeVector` (.x (.location (`SplineComponent.GetTransformAtSplinePoint` (`self.Spline`) (`self.StartLocation`) "World" false))) (.y (.location (`SplineComponent.GetTransformAtSplinePoint` (`self.Spline`) (`self.StartLocation`) "World" false))) (+ (.z (.location (`SplineComponent.GetTransformAtSplinePoint` (`self.Spline`) (`self.StartLocation`) "World" false))) (`local.FinishHalfHeight`))) (`KismetMathLibrary.MakeRotator` (.roll (.rotation (`SplineComponent.GetTransformAtSplinePoint` (`self.Spline`) (`self.StartLocation`) "World" false))) (.pitch (.rotation (`SplineComponent.GetTransformAtSplinePoint` (`self.Spline`) (`self.StartLocation`) "World" false))) (.yaw (.rotation (`SplineComponent.GetTransformAtSplinePoint` (`self.Spline`) (`self.StartLocation`) "World" false)))) false false)))))