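; Procedural decoration actor that scatters a configurable number of static mesh components around itself.
; ProceduralDeco loops NumOfMeshs times, adding a mesh at a random XY offset derived from unit vectors scaled by ModDistance, with Z at zero.
; It runs from both the construction script and BeginPlay without a seed or clearing step, so BeginPlay adds another randomly placed set.
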(event `self.ReceiveBeginPlay`
  (`self.Procedural Deco`))

(fn `Procedural Deco`
  (for _ (range 1 (+ (`self.Num of meshs`) 1))
    (`AddComponent|NODE_AddStaticMeshComponent-0` :`RelativeTransform` (`KismetMathLibrary.Conv_VectorToTransform` (`KismetMathLibrary.MakeVector` (.x (* (`KismetMathLibrary.RandomUnitVector`) (`self.Mod Distance`))) (.y (* (`KismetMathLibrary.RandomUnitVector`) (`self.Mod Distance`))))))))

(fn `UserConstructionScript`
  (`self.Procedural Deco`))