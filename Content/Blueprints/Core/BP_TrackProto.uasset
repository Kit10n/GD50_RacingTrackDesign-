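; BP_TrackProto is a prototype track actor that builds a mesh track along a spline in its construction script, with no active runtime logic.
; A distance loop adds spline mesh components with a configurable mesh and optional collision, plus a billboard at each step.
; Segments span SplineMeshLength but advance by a third of it, so they overlap.
; The tangent lookups and mesh-bounds length calculation are left unconnected.
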(fn `UserConstructionScript`
  (bind _spline (`self.Spline`))
  (bind _returnvalue (`KismetMathLibrary.Conv_VectorToTransform` (`SplineComponent.GetLocationAtDistanceAlongSpline` (`self.Spline`) (`self.CurrentSplineDistance`) "Local")))
  (`|ExecutionSequence`
    (:`then_0`)
    (:`then_1`
      (while (< (`self.CurrentSplineDistance`) (`SplineComponent.GetSplineLength` (`self.Spline`)))
        (bind _returnvalue_2 (`AddComponent|NODE_AddSplineMeshComponent-0` :`RelativeTransform` _returnvalue))
        (`AddComponent|NODE_AddBillboardComponent-0` :`RelativeTransform` _returnvalue)
        (`SplineMeshComponent.SetStartAndEnd` _returnvalue_2 (`SplineComponent.GetLocationAtDistanceAlongSpline` _spline (`self.CurrentSplineDistance`) "Local") (0.0 0.0 0.0) (`SplineComponent.GetLocationAtDistanceAlongSpline` _spline (+ (`self.CurrentSplineDistance`) (`self.SplineMeshLength`)) "Local") (0.0 0.0 0.0) true)
        (`StaticMeshComponent.SetStaticMesh` _returnvalue_2 (`self.Mesh`))
        (set `self.CurrentSplineDistance` (+ (`self.CurrentSplineDistance`) (/ (`self.SplineMeshLength`) 3.0)))
        (`PrimitiveComponent.SetCollisionEnabled` _returnvalue_2 (select `bool` (`self.TrackCollision`) :`false` "NoCollision" :`true` "QueryAndPhysics" :!type "ECollisionEnabled Enum"))))))